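; BP_Darts is an AI-driven creature, apparently a dragon, that interacts with the VR player and meat feed actors.
; Perception updates attempt to send it toward feed meat, and touching the VR pawn's Sphere1 spawns a heart Niagara effect.
; Random patrol, player-follow and see-pawn chase events exist, but their triggers are disconnected here.
; BeginPlay and Tick are empty, and HandleSIGHT only filters stimuli without acting.
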(event OnPerceptionUpdated(ActorSensing)
  (params (UpdatedActors :type Array%20of%20Actor%20Object%20References))
  (EventDispatchers|AssignOnActorBeginOverlap UpdatedActors (delegate Custom|OnActorBeginOverlap_Event))
  (bind _asseoyoung_actors (Utilities|Casting|CastToSeoyoung_Actors (stale Custom|OnActorBeginOverlap_Event OverlappedActor)))
  (bind _asfeed_meat (Utilities|Casting|CastTofeed_meat _asseoyoung_actors))
  (AI|Navigation|MovetoActor (AI|GetAIController self) _asfeed_meat -1.0 true true true 0)
  (Variables|/Script/Engine.CharacterMovementComponent|SetMaxAcceleration (Variables|Character|GetCharacterMovement) 3.5e+02)
  (Development|PrintString "dkaskdakdkasdak"))

(event OnTargetPerceptionUpdated(AIPerception)
  (params (Actor :type Actor%20Object%20Reference) (Stimulus :type AI%20Stimulus%20Structure)))

(event OnComponentBeginOverlap(Sphere)
  (params (OverlappedComponent :type Primitive%20Component%20Object%20Reference) (OtherActor :type Actor%20Object%20Reference) (OtherComp :type Primitive%20Component%20Object%20Reference) (OtherBodyIndex :type Integer) (bFromSweep :type Boolean) (SweepResult :type Hit%20Result%20Structure%20%28by%20ref%29))
  (bind _asvrpawn (Utilities|Casting|CastToVRPawn OtherActor))
  (if (== OtherComp (Variables|/Game/VRTemplate/Blueprints/VRPawn.VRPawn_C|GetSphere1 _asvrpawn))
    (Niagara|SpawnSystematLocation "/Game/seoyoung/Particle/NS_Heart.NS_Heart" (Transformation|GetWorldLocation (Variables|/Game/VRTemplate/Blueprints/VRPawn.VRPawn_C|GetSphere1 _asvrpawn)))))

(event Custom|Random%20Patrol
  (AI|AIMoveTo self (.RandomLocation (AI|Navigation|GetRandomReachablePointinRadius (Transformation|GetActorLocation) 1.5e+03 0 0)) 0 5.0 false
    (:then
      (Utilities|FlowControl|Delay 1.0)
      (bind _outactors (Actor|GetAllActorsOfClass "/Game/VRTemplate/Blueprints/VRPawn.VRPawn_C"))
      (if (not (Variables|/Game/VRTemplate/Blueprints/VRPawn.VRPawn_C|Getpatrol (Utilities|Array|Get(acopy) _outactors)))
        (CallFunction|RandomPatrol)))))

(event Custom|OnSeePawn_Event
  (params (Pawn :type Pawn%20Object%20Reference))
  (bind _asvrpawn (Utilities|Casting|CastToVRPawn Pawn))
  (bind _output_get (Variables|Default|SetPatrolTarget _asvrpawn))
  (AI|Navigation|MovetoActor (AI|GetAIController self) _output_get -1.0 true true true 0)
  (Variables|/Script/Engine.CharacterMovementComponent|SetMaxAcceleration (Variables|Character|GetCharacterMovement) 3.5e+02))

(event Custom|playertarget
  (bind _outactors (Actor|GetAllActorsOfClass "/Game/VRTemplate/Blueprints/VRPawn.VRPawn_C"))
  (AI|Navigation|MovetoActor (AI|GetAIController self) (Utilities|Array|Get(acopy) _outactors) -1.0 true true true 0)
  (Utilities|FlowControl|Delay 2.0))

(event Custom|OnActorBeginOverlap_Event
  (params (OverlappedActor :type Actor%20Object%20Reference) (OtherActor :type Actor%20Object%20Reference)))

(event EventBeginPlay)

(event Collision|EventActorBeginOverlap
  (params (OtherActor :type Actor%20Object%20Reference)))

(event EventTick
  (params (DeltaSeconds :type Float%20%28single-precision%29)))

(event Input|KeyboardEvents|E
  (params (Key :type Key%20Structure :default "None")))

(fn ConstructionScript)

(fn HandleSIGHT
  (params (ACTOR :type Actor%20Object%20Reference) (STIMULUS :type AI%20Stimulus%20Structure))
  (bind _returnvalue (Class|AIPerceptionSystem|GetSenseClassforStimulus STIMULUS))
  (if (== _returnvalue "/Script/AIModule.AISenseConfig_Sight")
    (if (not (== ACTOR "/Game/seoyoung/feed/gril_chiken_Cube.gril_chiken_Cube"))
      (return))
    (else
      (return))))